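; Combat playground actor that spawns random enemies when play begins.
; SpawnRandomEnemys loops over five spawn-point components and spawns a class picked at random from EnemysList at each one's world transform.
; Picks are independent per point, so the same enemy type can appear several times.
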(event `self.ReceiveBeginPlay`
  (`self.SpawnRandomEnemys`))

(fn `SpawnRandomEnemys`
  (for _array_element (`|MakeArray` (`self.spawn4`) (`self.spawn3`) (`self.spawn2`) (`self.spawn1`) (`self.spawn5`))
    (`|SpawnActorFromClass` (`KismetArrayLibrary.Array_Random` (`self.enemysList`)) (`SceneComponent.K2_GetComponentToWorld` _array_element) "Undefined" "MultiplyWithRoot" null null)))

(fn `UserConstructionScript`)