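; Combat playground actor that spawns the player's heroes at up to three spawn points.
; GetSetHeroPosition stores a map whose values are hero classes to spawn.
; CombatSpawn loops over the map's keys and spawns each class at the Spawn1, Spawn2 or Spawn3 component's world transform.
; The spawn point follows the loop index, so placement depends on map order rather than on the key itself.
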(event `self.ReceiveBeginPlay`)

(event `/Game/interfaces/BPI_combatHeroPosition.GetSetHeroPosition`
  (params (heroPositions :type "Map of Integer to /Game/blueprints/characters/heroes/BP_heroBase Class Reference"))
  (set `self.heroPositions` heroPositions))

(event `/Game/interfaces/BPI_spawn.CombatSpawn`
  (bind _heropositions (`self.heroPositions`))
  (bind _keys (`BlueprintMapLibrary.Map_Keys` _heropositions))
  (for (_array_element _array_index) _keys
    (`|SpawnActorFromClass` (`BlueprintMapLibrary.Map_Find` _heropositions _array_element) (`SceneComponent.K2_GetComponentToWorld` (select `int` _array_index :`0` (`self.spawn1`) :`1` (`self.spawn2`) :`2` (`self.spawn3`))) "Undefined" "MultiplyWithRoot" null null)))

(fn `UserConstructionScript`)