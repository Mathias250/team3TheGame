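; Test teleport trigger that sends the player from exploration into the combat test level and restores their position afterwards.
; On first capsule overlap by the player, it saves the character transform and used flag to a save slot, then opens the level.
; On BeginPlay it loads any such save, restores the flag and transform, then deletes the slot, so the trigger does not refire.
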(event `self.ReceiveBeginPlay`
  (bind _returnvalue (`GameplayStatics.DoesSaveGameExist` "explorationSave1"))
  (if _returnvalue
    (bind _returnvalue_2 (`GameplayStatics.LoadGameFromSlot` "explorationSave1"))
    (bind _assg_exploration_status_save (cast `/Game/blueprints/gameSaving/SG_explorationStatusSave` _returnvalue_2))
    (set `self.isUsed` (`/Game/blueprints/gameSaving/SG_explorationStatusSave.teleportStatus` _assg_exploration_status_save))
    (`self.K2_SetActorTransform` (`GameplayStatics.GetPlayerCharacter` 0) (`/Game/blueprints/gameSaving/SG_explorationStatusSave.characterPos` _assg_exploration_status_save) false false)
    (`GameplayStatics.DeleteGameInSlot` "explorationSave1")
    (`KismetSystemLibrary.PrintString` "Hello1")
    (else
      (`KismetSystemLibrary.PrintString` "Hello"))))

(event `self.Capsule.OnComponentBeginOverlap`
  (params (OverlappedComponent :type "PrimitiveComponent Object Reference") (OtherActor :type "Actor Object Reference") (OtherComp :type "PrimitiveComponent Object Reference") (OtherBodyIndex :type Integer) (bFromSweep :type Boolean) (SweepResult :type "HitResult Structure (by ref)"))
  (if (`self.isUsed`)
    _
    (elif (== OtherActor (`GameplayStatics.GetPlayerCharacter` 0))
      (set `self.isUsed` true)
      (bind _returnvalue (`GameplayStatics.CreateSaveGameObject` "/Game/blueprints/gameSaving/SG_explorationStatusSave.SG_explorationStatusSave_C"))
      (set `/Game/blueprints/gameSaving/SG_explorationStatusSave.characterPos` (`self.GetTransform` (`GameplayStatics.GetPlayerCharacter` 0)) _returnvalue)
      (set `/Game/blueprints/gameSaving/SG_explorationStatusSave.teleportStatus` (`self.isUsed`) _returnvalue)
      (`GameplayStatics.SaveGameToSlot` _returnvalue "explorationSave1")
      (`GameplayStatics.OpenLevel` "L_testCombatLevel")
      (else
        (`KismetSystemLibrary.PrintString` "Hello")))))

(fn `UserConstructionScript`)