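; BP_enemyBase is a base enemy character that holds combat stats (HP, max HP, agility, armor, name) and supports click selection.
; Clicking its capsule broadcasts the selection to every BP_enemyBase, so each updates its own selected flag.
; The selected enemy pushes its stats to top-level BW_combatBase widgets.
; SetStartStats initializes the stats, starting HP at maximum.
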(event `self.ReceiveBeginPlay`)

(event `self.ReceiveTick`
  (params (DeltaSeconds :type "Float (single-precision)")))

(event `self.CapsuleComponent.OnClicked`
  (params (TouchedComponent :type "PrimitiveComponent Object Reference") (ButtonPressed :type "Key Structure"))
  (bind _outactors (`GameplayStatics.GetAllActorsOfClass` "BP_enemyBase_C"))
  (for _array_element _outactors
    (`self.GetSetEnemy` _array_element self)))

(event `/Game/interfaces/BPI_selectedEnemy.GetSetEnemy`
  (params (SelectedEnemy :type "/Game/blueprints/characters/enemys/BP_enemyBase Object Reference"))
  (bind _output_get (set `self.combatEnemyIsSelected` (== SelectedEnemy self)))
  (if _output_get
    (bind _foundwidgets (`WidgetBlueprintLibrary.GetAllWidgetsOfClass` "/Game/uis/combatUis/BW_combatBase.BW_combatBase_C"))
    (`/Game/interfaces/BPI_enemyStats.GetEnemyStats` _foundwidgets (`self.hp`) (`self.maxHp`) (`self.agility`) (`self.armor`) (`self.name`))))

(fn `SetStartStats`
  (params (startHP :type Integer) (startAgility :type Integer) (startArmor :type Integer) (startName :type String))
  (bind _output_get (set `self.maxHp` startHP))
  (set `self.hp` _output_get)
  (set `self.agility` startAgility)
  (set `self.armor` startArmor)
  (set `self.name` startName))

(fn `UserConstructionScript`)