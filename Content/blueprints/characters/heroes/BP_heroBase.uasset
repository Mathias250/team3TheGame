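; Base hero for combat, holding HP, agility, armor and three abilities, with setup functions for starting values.
; Hovering selects the hero, notifying every hero and the game mode, and the selected one pushes its stats to the combat widget.
; Clicking a targetable hero reports it to the game mode as the ability target.
; Capped heals and buffs, and damage, also reselect the hero to refresh the display; death notifies the game mode and destroys the actor.
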(event `self.ReceiveBeginPlay`)

(event `self.ReceiveTick`
  (params (DeltaSeconds :type "Float (single-precision)")))

(event `self.CapsuleComponent.OnBeginCursorOver`
  (params (TouchedComponent :type "PrimitiveComponent Object Reference"))
  (`self.SetSelectedHero`))

(event `GetSetHero_1`
  (params (SelectedHero :type "/Game/blueprints/characters/heroes/BP_heroBase Object Reference"))
  (bind _output_get (set `self.combatIsSelected` (== SelectedHero self)))
  (if _output_get
    (bind _foundwidgets (`WidgetBlueprintLibrary.GetAllWidgetsOfClass` "/Game/uis/combatUis/BW_combatBase.BW_combatBase_C"))
    (message `/Game/interfaces/BPI_heroStats.GetHeroStats` _foundwidgets (`self.hp`) (`self.maxHp`) (`self.agility`) (`self.armor`) (`self.name`) (`self.abilities`))))

(event `self.CapsuleComponent.OnClicked`
  (params (TouchedComponent :type "PrimitiveComponent Object Reference") (ButtonPressed :type "Key Structure"))
  (if (`self.heroCanBeTargeted`)
    (message `/Game/interfaces/BPI_setAbilityTargetHero.GetSetAbilityTargetHero` (`GameplayStatics.GetGameMode`) self)))

(event `/Game/interfaces/BPI_buffHero.HealHero`
  (params (value :type Integer))
  (bind _returnvalue (+ (`self.hp`) value))
  (if (> _returnvalue (`self.maxHp`))
    (set `self.hp` (`self.maxHp`))
    (else
      (set `self.hp` _returnvalue)))
  (`self.SetSelectedHero` :!label _label))

(event `/Game/interfaces/BPI_buffHero.BuffHeroAgility`
  (params (value :type Integer))
  (bind _returnvalue (+ (`self.agility`) value))
  (if (> _returnvalue 100)
    (set `self.agility` 100)
    (goto _label)
    (else
      (set `self.agility` _returnvalue)
      (goto _label))))

(event `/Game/interfaces/BPI_buffHero.BuffHeroArmor`
  (params (value :type Integer))
  (bind _returnvalue (+ (`self.armor`) value))
  (if (> _returnvalue 100)
    (set `self.armor` 100)
    (goto _label)
    (else
      (set `self.armor` _returnvalue)
      (goto _label))))

(event `/Game/interfaces/BPI_heroDamage.DamageHero`
  (params (damageValue :type Integer) (isAP :type Boolean))
  (bind _output_get (set `self.hp` (- (`self.hp`) damageValue)))
  (`self.SetSelectedHero`)
  (if (< _output_get 1)
    (message `/Game/interfaces/BPI_heroDied.heroDied` (`GameplayStatics.GetGameMode`) self)
    (`self.K2_DestroyActor`)))

(fn `SetSelectedHero`
  (bind _outactors (`GameplayStatics.GetAllActorsOfClass` "BP_heroBase_C"))
  (for _array_element _outactors
    (`self.GetSetHero` _array_element self))
  (message `/Game/interfaces/BPI_selectedHero.GetSetHero` (`GameplayStatics.GetGameMode`) self))

(fn `SetStartAbilities`
  (params (ability1 :type "/Game/blueprints/characters/heroes/S_abilityStructure Structure") (ability2 :type "/Game/blueprints/characters/heroes/S_abilityStructure Structure") (ability3 :type "/Game/blueprints/characters/heroes/S_abilityStructure Structure"))
  (bind _abilities (`self.abilities`))
  (bind _output_get (set `self.ability1` ability1))
  (`KismetArrayLibrary.Array_Add` _abilities _output_get)
  (bind _output_get_2 (set `self.ability2` ability2))
  (`KismetArrayLibrary.Array_Add` _abilities _output_get_2)
  (bind _output_get_3 (set `self.ability3` ability3))
  (`KismetArrayLibrary.Array_Add` _abilities _output_get_3))

(fn `SetStartStats`
  (params (startHP :type Integer) (startAgility :type Integer) (startArmor :type Integer) (name :type String))
  (bind _output_get (set `self.maxHp` startHP))
  (set `self.hp` _output_get)
  (set `self.agility` startAgility)
  (set `self.armor` startArmor)
  (set `self.name` name))

(fn `UserConstructionScript`)